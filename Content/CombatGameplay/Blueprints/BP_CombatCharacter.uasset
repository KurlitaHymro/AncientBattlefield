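; Player combat character Blueprint that builds the HUD and inventory UI on BeginPlay.
; It creates the player layout widget, gives its state bar the combat ability system component, and binds four ability slots to that component and the abilities input component.
; It then adds an inventory layout fed by the inventory and equipment components and shows the mouse cursor.
; Older separate inventory and equipment widgets with visibility toggles remain as unconnected nodes.
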(event `Key|I`
  (params (Key :type "Key Structure")))

(event `Key|C`
  (params (Key :type "Key Structure")))

(event `self.ReceiveBeginPlay`
  (`|ExecutionSequence`
    (:`then_0`
      (bind _returnvalue (`|CreateWidget` "/Game/CombatGameplay/Widget/WB_Player_Layout.WB_Player_Layout_C"))
      (bind _output_get (set `self.StateLayout` _returnvalue))
      (`UserWidget.AddToViewport` _output_get 0)
      (`self.InitializationStateBar`)
      (`self.InitialzationAbilitiesInfo`))
    (:`then_3`
      (bind _returnvalue_2 (`|CreateWidget` "/Game/ItemInventorySystem/Widget/WB_InventoryLayout.WB_InventoryLayout_C" null (`self.InventoryComponent`) (`self.EquipmentComponent`)))
      (`UserWidget.AddToViewport` _returnvalue_2 0)
      (set `PlayerController.bShowMouseCursor` true (cast `PlayerController` (`self.GetController`) :!pure true)))))

(fn `UserConstructionScript`)