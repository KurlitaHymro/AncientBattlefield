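; BP_PlayerCharacter is the player character Blueprint that sets up the HUD and inventory UI for combat gameplay.
; BeginPlay creates the player layout and passes CombatAbilityComponent to its state bar as the ability system source.
; It also creates a hidden inventory layout, binding its inventory and equipment panels to their components before running each component's Setup.
; The I key flip-flops the inventory layout's visibility together with the mouse cursor.
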(event `self.ReceiveBeginPlay`
  (bind _inventorywidget (`self.InventoryWidget`))
  (`|ExecutionSequence`
    (:`then_0`
      (bind _returnvalue (`|CreateWidget` "/Game/CombatGameplay/Widget/WB_Player_Layout.WB_Player_Layout_C"))
      (`UserWidget.AddToViewport` _returnvalue 0)
      (set `/Game/CombatGameplay/Widget/WB_Player_StateBar.AbilitySystemComponent` (`self.CombatAbilityComponent`) (`/Game/CombatGameplay/Widget/WB_Player_Layout.WB_Player_StateBar` _returnvalue)))
    (:`then_1`
      (bind _returnvalue_2 (`|CreateWidget` "/Game/ItemInventoryGameplay/Widget/WB_Player_Inventory_Layout.WB_Player_Inventory_Layout_C"))
      (bind _output_get (set `self.InventoryWidget` _returnvalue_2))
      (`UserWidget.AddToViewport` _output_get 0)
      (`Widget.SetVisibility` _output_get "Hidden")
      (`|ExecutionSequence`
        (:`then_0`
          (`/Game/ItemInventoryGameplay/Widget/WB_Player_Inventory.BindEvent` (`/Game/ItemInventoryGameplay/Widget/WB_Player_Inventory_Layout.WB_Player_Inventory` _inventorywidget) (`self.InventoryComponent`))
          (`InventoryComponent.Setup` (`self.InventoryComponent`) 35))
        (:`then_1`
          (`/Game/ItemInventoryGameplay/Widget/WB_Player_Equipment.BindEvent` (`/Game/ItemInventoryGameplay/Widget/WB_Player_Inventory_Layout.WB_Player_Equipment` _inventorywidget) (`self.EquipmentComponent`))
          (`InventoryComponent.Setup` (`self.EquipmentComponent`) 0))))))

(event `Key|I`
  (params (Key :type "Key Structure"))
  (bind _inventorywidget (`self.InventoryWidget`))
  (bind `_as玩家控制器` (cast `PlayerController` (`self.GetController`) :!pure true))
  (:`Pressed`
    (`/Engine/EditorBlueprintResources/StandardMacros.FlipFlop`
      (:`A`
        (`Widget.SetVisibility` _inventorywidget "Visible")
        (set `PlayerController.bShowMouseCursor` true `_as玩家控制器`))
      (:`B`
        (`Widget.SetVisibility` _inventorywidget "Hidden")
        (set `PlayerController.bShowMouseCursor` false `_as玩家控制器`)))))

(fn `UserConstructionScript`)