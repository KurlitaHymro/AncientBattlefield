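; Player controller for the combat gameplay mode that owns the in-game HUD and main menu widgets.
; On BeginPlay it creates the playing layout and main menu and adds both to the viewport, with the menu starting hidden.
; Tab alternates through a FlipFlop between showing the menu with the mouse cursor and hiding both, without changing input mode.
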(event `self.ReceiveBeginPlay`
  (`self.CreateLayout`)
  (`self.CreateMainMenu`))

(event `Key|Tab`
  (params (Key :type "Key Structure"))
  (bind _mainmenu (`self.MainMenu`))
  (:`Pressed`
    (`/Engine/EditorBlueprintResources/StandardMacros.FlipFlop`
      (:`A`
        (`Widget.SetVisibility` _mainmenu "Visible")
        (set `PlayerController.bShowMouseCursor` true))
      (:`B`
        (`Widget.SetVisibility` _mainmenu "Hidden")
        (set `PlayerController.bShowMouseCursor` false)))))

(fn `UserConstructionScript`)