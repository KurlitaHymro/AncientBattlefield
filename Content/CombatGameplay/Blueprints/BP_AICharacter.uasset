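; BP_AICharacter is an AI combat character that arms itself with a two-handed greatsword shortly after spawning.
; BeginPlay links the overhead state-bar widget to the character's CombatAbilityComponent and sets up its inventory and equipment components.
; After a short delay, it creates the sword item from a named prefab, adds it to the inventory and puts it on through the item's equipment property fragment.
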(event `self.ReceiveBeginPlay`
  (`|ExecutionSequence`
    (:`then_0`
      (set `/Game/CombatGameplay/Widget/WB_Head_StateBar.AbilitySystemComponent` (`self.CombatAbilityComponent`) (cast `/Game/CombatGameplay/Widget/WB_Head_StateBar` (`WidgetComponent.GetUserWidgetObject` (`self.Widget`)) :!pure true)))
    (:`then_1`
      (`|ExecutionSequence`
        (:`then_0`
          (`InventoryComponent.Setup` (`self.InventoryComponent`) 10))
        (:`then_1`
          (`InventoryComponent.Setup` (`self.EquipmentComponent`) 0))
        (:`then_2`
          (`KismetSystemLibrary.Delay` 3.0)
          (bind _returnvalue (`InventoryItemConfig.NewInventoryItem` self "双手大剑"))
          (`InventoryComponent.AddItem` (`self.InventoryComponent`) _returnvalue 0)
          (bind _returnvalue_2 (`ItemObject.FindPropertyFragment` _returnvalue "/Script/AncientBattlefield.PropertyFragment_Equipment"))
          (bind _asproperty_fragment_equipment (cast `PropertyFragment_Equipment` _returnvalue_2))
          (`PropertyFragment_Equipment.PutOn` _asproperty_fragment_equipment))))))

(fn `UserConstructionScript`)